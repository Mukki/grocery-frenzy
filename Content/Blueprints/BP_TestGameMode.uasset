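; BP_TestGameMode is a game mode for a timed score-target game, showing the in-game UI on BeginPlay.
; Tick uses a one-second Delay to decrement TimeRemaining, calling EndGame when it runs out.
; IncreaseScore increments and prints Score, also calling EndGame at the hard-coded target.
; EndGame pauses the game, replaces all widgets with the end menu and enables the mouse cursor with Game and UI input.
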(event EventBeginPlay
  (bind _returnvalue (UserInterface|CreateWidget "/Game/UI/WB_IngameUI.WB_IngameUI_C"))
  (UserInterface|Viewport|AddtoViewport _returnvalue 0))

(event EventTick
  (params (DeltaSeconds :type Float%20%28single-precision%29))
  (Utilities|FlowControl|Delay 1.0)
  (Variables|Default|SetTimeRemaining (- (Variables|Default|GetTimeRemaining) 1))
  (if (<= (Variables|Default|GetTimeRemaining) 0)
    (CallFunction|EndGame)))

(fn ConstructionScript)

(fn IncreaseScore
  (bind _output_get (Variables|Default|SetScore (+ (Variables|Default|GetScore) 1)))
  (Development|PrintString (Utilities|String|ToString(Integer) _output_get))
  (if (>= _output_get 10)
    (CallFunction|EndGame)))

(fn EndGame
  (bind _returnvalue (Game|GetPlayerController 0))
  (Game|SetGamePaused true)
  (Viewport|RemoveAllWidgets)
  (bind _returnvalue_2 (UserInterface|CreateWidget "/Game/UI/WB_EndMenu.WB_EndMenu_C"))
  (UserInterface|Viewport|AddtoViewport _returnvalue_2 0)
  (Input|SetInputModeGameandUI _returnvalue 0 "DoNotLock" true false)
  (Variables|/Script/Engine.PlayerController|SetbShowMouseCursor _returnvalue true))