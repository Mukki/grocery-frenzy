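; Player character that grabs, drops, throws and interacts with nearby objects.
; InteractionBox overlaps maintain lists of in-range actors implementing BPI_Grabbable or BPI_Interactable, and input actions act on the first entry of each.
; Grab attaches the item supplied by the grabbable to HeldItemLocation, while a second press detaches it and notifies it.
; Throw also detaches and notifies it, then adds a forward impulse scaled by ThrowingStrength.
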(event Custom|OnInteractionBoxBeginOverlap
  (params (OverlappedComponent :type Primitive%20Component%20Object%20Reference) (OtherActor :type Actor%20Object%20Reference) (OtherComp :type Primitive%20Component%20Object%20Reference) (OtherBodyIndex :type Integer) (bFromSweep :type Boolean) (SweepResult :type Hit%20Result%20Structure%20%28by%20ref%29))
  ;[0.4078 0.4196 1] Ajoute les objets interactifs proches à une liste
  (if (== OverlappedComponent (Variables|Default|GetInteractionBox))
    (if (Utilities|DoesObjectImplementInterface OtherActor "/Game/Blueprints/Items/BPI_Grabbable.BPI_Grabbable_C")
      (Utilities|Array|AddUnique (Variables|Default|GetGrabbablesInRange) OtherActor))
    (if (Utilities|DoesObjectImplementInterface OtherActor "/Game/Blueprints/Items/BPI_Interactable.BPI_Interactable_C")
      (Utilities|Array|AddUnique (Variables|Default|GetInteractablesInRange) OtherActor))))

(event Custom|OnInteractionBoxEndOverlap
  (params (OverlappedComponent :type Primitive%20Component%20Object%20Reference) (OtherActor :type Actor%20Object%20Reference) (OtherComp :type Primitive%20Component%20Object%20Reference) (OtherBodyIndex :type Integer))
  ;[0.4078 0.4196 1] Retire les objets des listes lorsqu'ils sont hors de portée
  (if (== OverlappedComponent (Variables|Default|GetInteractionBox))
    (Utilities|Array|RemoveItem (Variables|Default|GetGrabbablesInRange) OtherActor)
    (Utilities|Array|RemoveItem (Variables|Default|GetInteractablesInRange) OtherActor)))

(event Input|EnhancedActionEvents|EnhancedInputActionBP_GrabIA
  (params (ActionValue :type Boolean) (ElapsedSeconds :type Float%20%28double-precision%29) (TriggeredSeconds :type Float%20%28double-precision%29) (InputAction :type Input%20Action%20Object%20Reference :default "/Game/Blueprints/Character/Input/BP_GrabIA.BP_GrabIA"))
  (bind _grabbablesinrange (Variables|Default|GetGrabbablesInRange))
  ;[1 0.4877 0] Grab / lacher un objet
  (if (Utilities|IsValid (Variables|Default|GetHeldItem))
    ;;[1 1 1] Lacher un objet
    (Development|PrintText "Drop" true true "(R=0.072942,G=1.000000,B=0.000000,A=1.000000)")
    (Transformation|DetachFromActor (Variables|Default|GetHeldItem) "KeepWorld" "KeepWorld" "KeepWorld")
    (Class|BPIGrabbable|OnDrop(Message) (Variables|Default|GetHeldItem))
    (Variables|Default|SetHeldItem 0)
    (else
      ;;[1 1 1] Attraper objet
      (Development|PrintText "Grab" true true "(R=0.072942,G=1.000000,B=0.000000,A=1.000000)")
      (if (Utilities|Array|IsNotEmpty _grabbablesinrange)
        (bind _itemtograb (Class|BPIGrabbable|GetItemtoGrab(Message) (Utilities|Array|Get(acopy) _grabbablesinrange)))
        (Class|BPIGrabbable|OnGrab(Message) _itemtograb)
        (Transformation|AttachComponentToComponent _itemtograb (Variables|Default|GetHeldItemLocation) "None" "SnapToTarget" "SnapToTarget" "KeepWorld" true)
        (Variables|Default|SetHeldItem _itemtograb)))))

(event Input|EnhancedActionEvents|EnhancedInputActionBP_InteractIA
  (params (ActionValue :type Boolean) (ElapsedSeconds :type Float%20%28double-precision%29) (TriggeredSeconds :type Float%20%28double-precision%29) (InputAction :type Input%20Action%20Object%20Reference :default "/Game/Blueprints/Character/Input/BP_InteractIA.BP_InteractIA"))
  (bind _interactablesinrange (Variables|Default|GetInteractablesInRange))
  ;[0.07661 1 0.3525] Interaction
  (Development|PrintText "Interact" true true "(R=0.072942,G=1.000000,B=0.000000,A=1.000000)")
  (if (Utilities|Array|IsNotEmpty _interactablesinrange)
    (Class|BPIInteractable|Interact(Message) (Utilities|Array|Get(acopy) _interactablesinrange) self)))

(event Input|EnhancedActionEvents|EnhancedInputActionBP_ThrowIA
  (params (ActionValue :type Boolean) (ElapsedSeconds :type Float%20%28double-precision%29) (TriggeredSeconds :type Float%20%28double-precision%29) (InputAction :type Input%20Action%20Object%20Reference :default "/Game/Blueprints/Character/Input/BP_ThrowIA.BP_ThrowIA"))
  (if (Utilities|IsValid (Variables|Default|GetHeldItem))
    (Development|PrintText "Throw" true true "(R=0.072942,G=1.000000,B=0.000000,A=1.000000)")
    (Transformation|DetachFromActor (Variables|Default|GetHeldItem) "KeepWorld" "KeepWorld" "KeepWorld")
    (Class|BPIGrabbable|OnDrop(Message) (Variables|Default|GetHeldItem))
    (Physics|AddImpulse (Actor|GetComponentbyClass (Variables|Default|GetHeldItem) "/Script/Engine.PrimitiveComponent") (* (Math|Vector|GetForwardVector (Transformation|GetActorRotation)) (Variables|Default|GetThrowingStrength)) "None" false)
    (Variables|Default|SetHeldItem 0)))

(event EventBeginPlay
  ;[1 1 1] Initialisation
  (Collision|BindEventtoOnComponentEndOverlap (Variables|Default|GetInteractionBox) (delegate Custom|OnInteractionBoxEndOverlap))
  (Collision|AssignOnComponentBeginOverlap (Variables|Default|GetInteractionBox) (delegate Custom|OnInteractionBoxBeginOverlap)))

(event Collision|EventActorBeginOverlap
  (params (OtherActor :type Actor%20Object%20Reference)))

(event EventTick
  (params (DeltaSeconds :type Float%20%28single-precision%29)))

(fn ConstructionScript)