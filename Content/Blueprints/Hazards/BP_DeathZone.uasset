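; Death zone hazard that respawns players who overlap it and cleans up anything else that falls in.
; On player overlap it destroys any held item, plays a plop sound, then destroys the character.
; A new character spawns at the PlayerStart indexed by player controller ID and is possessed by the same controller, relying on GetAllActorsOfClass order.
; Other overlapping actors get a short life span.
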(event EventBeginPlay)

(event Collision|EventActorBeginOverlap
  (params (OtherActor :type Actor%20Object%20Reference))
  (bind _asbp_player_character (Utilities|Casting|CastToBP_PlayerCharacter OtherActor)
    (:then
      (if (Utilities|IsValid (Variables|/Game/Blueprints/Character/BP_PlayerCharacter.BP_PlayerCharacter_C|GetHeldItem _asbp_player_character))
        (Actor|DestroyActor (Variables|/Game/Blueprints/Character/BP_PlayerCharacter.BP_PlayerCharacter_C|GetHeldItem _asbp_player_character)))
      (bind _asplayer_controller (Utilities|Casting|CastToPlayerController (Pawn|GetController _asbp_player_character)))
      (Audio|PlaySound2D "/Game/Assets/SFX/plopp-84863.plopp-84863" 0.7 1.0 0.0 0 0)
      (Actor|DestroyActor _asbp_player_character)
      (bind _outactors (Actor|GetAllActorsOfClass "/Script/Engine.PlayerStart"))
      (bind _returnvalue (Game|SpawnActorfromClass "/Game/Blueprints/Character/BP_PlayerCharacter.BP_PlayerCharacter_C" (Transformation|GetActorTransform (Utilities|Array|Get(acopy) _outactors (Class|GameplayStatics|GetPlayerControllerID _asplayer_controller))) "Undefined" "MultiplyWithRoot" 0 0))
      (Pawn|Possess _asplayer_controller _returnvalue))
    (:CastFailed
      (Actor|SetLifeSpan OtherActor 2.0))))

(event EventTick
  (params (DeltaSeconds :type Float%20%28single-precision%29)))

(fn ConstructionScript)