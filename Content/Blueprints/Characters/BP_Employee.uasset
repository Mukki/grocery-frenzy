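; Player-controlled employee character that moves on fixed world axes, carries products and interacts with nearby actors.
; Grab toggles between dropping HeldItem and picking the first BP_BaseProduct overlapping InteractionBox, which supplies the item to snap onto HeldItemBox.
; Interact sends a message, passing the employee, to the first actor overlapping InteractionBox.
; Message calls let each target handle its own grab, drop and interaction response.
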(event Input|ActionEvents|InputActionGrab
  (params (Key :type Key%20Structure :default "None"))
  (bind _interaction_box (Variables|Default|GetInteraction%20box))
  (bind _overlappingactors (Collision|GetOverlappingActors _interaction_box "/Game/Blueprints/Items/Products/BP_BaseProduct.BP_BaseProduct_C" :!class /Script/Engine.PrimitiveComponent))
  ;[1 0.4877 0] Grab / lacher un objet
  (:Pressed
    (if (Utilities|IsValid (Variables|Default|GetHeldItem))
      ;;[1 1 1] Lacher un objet
      (Development|PrintText "Drop" true true "(R=0.072942,G=1.000000,B=0.000000,A=1.000000)")
      (Transformation|DetachFromActor (Variables|Default|GetHeldItem) "KeepWorld" "KeepWorld" "KeepWorld")
      (Class|BPIGrabbable|OnDrop(Message) (Variables|Default|GetHeldItem))
      (Variables|Default|SetHeldItem 0)
      (else
        ;;[1 1 1] Attraper objet
        (Development|PrintText "Grab" true true "(R=0.072942,G=1.000000,B=0.000000,A=1.000000)")
        (if (Utilities|Array|IsNotEmpty _overlappingactors)
          (bind _itemtograb (Class|BPIGrabbable|GetItemtoGrab(Message) (Utilities|Array|Get(acopy) _overlappingactors)))
          (Class|BPIGrabbable|OnGrab(Message) _itemtograb)
          (Transformation|AttachComponentToComponent _itemtograb (Variables|Default|GetHeldItemBox) "None" "SnapToTarget" "SnapToTarget" "KeepWorld" true)
          (Variables|Default|SetHeldItem _itemtograb))))))

(event Input|ActionEvents|InputActionInterract
  (params (Key :type Key%20Structure :default "None"))
  (bind _interaction_box (Variables|Default|GetInteraction%20box))
  (bind _overlappingactors (Collision|GetOverlappingActors _interaction_box 0 :!class /Script/Engine.PrimitiveComponent))
  ;[0.07661 1 0.3525] Interaction
  (:Pressed
    (Development|PrintText "Interact" true true "(R=0.072942,G=1.000000,B=0.000000,A=1.000000)")
    (if (Utilities|Array|IsNotEmpty _overlappingactors)
      (Class|BPIInteractable|Interact(Message) (Utilities|Array|Get(acopy) _overlappingactors) self))))

(event Input|AxisEvents|InputAxisMoveForward/Backward
  (params (AxisValue :type Float%20%28single-precision%29))
  ;[1 1 1] Initialisation
  (Pawn|Input|AddMovementInput "0.000000,-1.000000,0.000000" AxisValue false))

(event Input|AxisEvents|InputAxisMoveRight/Left
  (params (AxisValue :type Float%20%28single-precision%29))
  ;[1 1 1] Initialisation
  (Pawn|Input|AddMovementInput "1.000000,0.000000,0.000000" AxisValue false))

(fn ConstructionScript)