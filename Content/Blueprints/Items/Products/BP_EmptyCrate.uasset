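; BP_EmptyCrate is a grabbable empty crate item that names itself "Crate vide" on BeginPlay.
; GetItemToGrab returns the crate itself as the object to pick up.
; OnGrab disables physics simulation and collision on its Box component, and OnDrop restores both.
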(event EventBeginPlay
  (Variables|Default|SetItemName "Crate vide"))

(event Collision|EventActorBeginOverlap
  (params (OtherActor :type Actor%20Object%20Reference)))

(event EventTick
  (params (DeltaSeconds :type Float%20%28single-precision%29)))

(fn ConstructionScript)

(fn GetItemtoGrab
  (return self))

(fn OnGrab
  (bind _box (Variables|Default|GetBox))
  (Physics|SetSimulatePhysics _box false)
  (Collision|SetCollisionEnabled _box "NoCollision")
  (return false))

(fn OnDrop
  (bind _box (Variables|Default|GetBox))
  (Physics|SetSimulatePhysics _box true)
  (Collision|SetCollisionEnabled _box "QueryAndPhysics")
  (return false))