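; BP_TomatoCrate is a tomato crate item that can be grabbed and dropped.
; GetItemToGrab returns the crate itself as the item to pick up.
; The grab event turns off physics simulation and collision on the Box component, and the drop event restores both.
; Separate OnGrab and OnDrop functions only return false, and the construction script is empty.
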(event Custom|OnDrop_1_1
  (bind _box (Variables|Default|GetBox))
  (Physics|SetSimulatePhysics _box true)
  (Collision|SetCollisionEnabled _box "QueryAndPhysics"))

(event Custom|OnGrab_1_1
  (bind _box (Variables|Default|GetBox))
  (Physics|SetSimulatePhysics _box false)
  (Collision|SetCollisionEnabled _box "NoCollision"))

(event EventBeginPlay)

(event Collision|EventActorBeginOverlap
  (params (OtherActor :type Actor%20Object%20Reference)))

(event EventTick
  (params (DeltaSeconds :type Float%20%28single-precision%29)))

(fn ConstructionScript)

(fn GetItemtoGrab
  (return self))

(fn OnDrop
  (return false))

(fn OnGrab
  (return false))