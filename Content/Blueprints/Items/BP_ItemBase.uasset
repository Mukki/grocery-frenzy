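; Base item actor that the player can grab and drop, highlighted when the player character is near.
; Box overlap events adjust a counter and toggle the mesh's custom depth for the highlight, with debug text.
; GetItemToGrab returns the actor itself; OnGrab turns off the box's physics and collision, and OnDrop restores them.
; DisableGravity, Tick and the construction script are empty.
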(event OnComponentBeginOverlap(Box)
  (params (OverlappedComponent :type Primitive%20Component%20Object%20Reference) (OtherActor :type Actor%20Object%20Reference) (OtherComp :type Primitive%20Component%20Object%20Reference) (OtherBodyIndex :type Integer) (bFromSweep :type Boolean) (SweepResult :type Hit%20Result%20Structure%20%28by%20ref%29))
  ;[1 1 1] highlight object
  (Utilities|Casting|CastToBP_PlayerCharacter OtherActor)
  (Math|Integer|IncrementInt (Variables|Default|Getlooking_at_veggie)
    (:%20%20
      (Development|PrintText "CLOSE")
      (Rendering|SetRenderCustomDepth (Variables|Default|GetStaticMesh) true))))

(event OnComponentEndOverlap(Box)
  (params (OverlappedComponent :type Primitive%20Component%20Object%20Reference) (OtherActor :type Actor%20Object%20Reference) (OtherComp :type Primitive%20Component%20Object%20Reference) (OtherBodyIndex :type Integer))
  ;[1 1 1] highlight object
  (Utilities|Casting|CastToBP_PlayerCharacter OtherActor)
  (bind _result (Math|Integer|DecrementInt (Variables|Default|Getlooking_at_veggie))
    (:%20%20
      (if (== _result 0)
        (Development|PrintText "FAR")
        (Rendering|SetRenderCustomDepth (Variables|Default|GetStaticMesh) false)))))

(event Collision|EventActorBeginOverlap
  (params (OtherActor :type Actor%20Object%20Reference)))

(event EventTick
  (params (DeltaSeconds :type Float%20%28single-precision%29)))

(fn ConstructionScript)

(fn DisableGravity)

(fn GetItemtoGrab
  (return self))

(fn OnDrop
  (bind _box (Variables|Default|GetBox))
  (Physics|SetSimulatePhysics _box true)
  (Collision|SetCollisionEnabled _box "QueryAndPhysics")
  (return false))

(fn OnGrab
  (bind _box (Variables|Default|GetBox))
  (Physics|SetSimulatePhysics _box false)
  (Collision|SetCollisionEnabled _box "NoCollision")
  (return false))