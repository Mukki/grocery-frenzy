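; Lettuce shelf that the player restocks from a crate and that hands out product items.
; Interact destroys a held crate of the matching class and refills the product count, otherwise printing a wrong-crate message.
; GetItemToGrab decrements the count and spawns a product at the world origin, while Tick shows display products only when stock remains.
; Box overlaps with the player drive a counter that toggles custom-depth highlighting on the mesh.
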(event OnComponentBeginOverlap(Box)
  (params (OverlappedComponent :type Primitive%20Component%20Object%20Reference) (OtherActor :type Actor%20Object%20Reference) (OtherComp :type Primitive%20Component%20Object%20Reference) (OtherBodyIndex :type Integer) (bFromSweep :type Boolean) (SweepResult :type Hit%20Result%20Structure%20%28by%20ref%29))
  ;[1 1 1] highlight object
  (Utilities|Casting|CastToBP_PlayerCharacter OtherActor)
  (Math|Integer|IncrementInt (Variables|Default|GetLooking%20At%20Shelf)
    (:%20%20
      (Development|PrintText "CLOSE")
      (Rendering|SetRenderCustomDepth (Variables|Default|GetStaticMesh) true)
      (Development|PrintText "render custom depth activated"))))

(event OnComponentEndOverlap(Box)
  (params (OverlappedComponent :type Primitive%20Component%20Object%20Reference) (OtherActor :type Actor%20Object%20Reference) (OtherComp :type Primitive%20Component%20Object%20Reference) (OtherBodyIndex :type Integer))
  ;[1 1 1] highlight object
  (Utilities|Casting|CastToBP_PlayerCharacter OtherActor)
  (bind _result (Math|Integer|DecrementInt (Variables|Default|GetLooking%20At%20Shelf))
    (:%20%20
      (if (== _result 0)
        (Development|PrintText "FAR")
        (Rendering|SetRenderCustomDepth (Variables|Default|GetStaticMesh) false)))))

(event Custom|OnDrop_1_1)

(event Custom|OnGrab_1_1)

(event EventBeginPlay)

(event Collision|EventActorBeginOverlap
  (params (OtherActor :type Actor%20Object%20Reference)))

(event EventTick
  (params (DeltaSeconds :type Float%20%28single-precision%29))
  (Rendering|SetVisibility (Variables|Default|GetDisplayProducts) (> (Variables|Default|GetProductCount) 0) true))

(event EventInteract
  (params (PlayerCharacter :type BP%20Player%20Character%20Object%20Reference))
  (if (== (Utilities|GetClass (Variables|/Game/Blueprints/Character/BP_PlayerCharacter.BP_PlayerCharacter_C|GetHeldItem PlayerCharacter)) (Variables|Default|GetCrateBPClass))
    (Audio|PlaySound2D "/Game/Sounds/SoundEffects/thump.thump" 1.0 1.0 0.0 0 0)
    (Actor|DestroyActor (Variables|/Game/Blueprints/Character/BP_PlayerCharacter.BP_PlayerCharacter_C|GetHeldItem PlayerCharacter))
    (Variables|/Game/Blueprints/Character/BP_PlayerCharacter.BP_PlayerCharacter_C|SetHeldItem PlayerCharacter 0)
    (Variables|Default|SetProductCount 3)
    (else
      (Development|PrintText "Pasl a bonne crate"))))

(fn ConstructionScript)

(fn GetItemtoGrab
  (if (> (Variables|Default|GetProductCount) 0)
    (Variables|Default|SetProductCount (- (Variables|Default|GetProductCount) 1))
    (bind _returnvalue (Game|SpawnActorfromClass (Variables|Default|GetProductBPClass) (Math|Transform|MakeTransform "0, 0, 0") "Undefined" "MultiplyWithRoot" 0 0))
    (return _returnvalue)
    (else
      (return 0))))

(fn OnDrop
  (return false))

(fn OnGrab
  (return false))