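; Customer spawner that keeps adding AI customers up to a cap, each with its own possessing controller and the spawner's location as its exit.
; It spawns one on BeginPlay, then Tick waits a delay whenever the area is clear, using the Overlapping flag as a gate.
; Each controller gets a random distinctive item from a pool, though removal rolls a separate index.
; FreeUsedItem returns items to the pool.
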(event EventBeginPlay
  (bind _usable_distinct_item (Variables|Default|GetUsable%20Distinct%20Item))
  (bind _box (Variables|Default|GetBox))
  (bind _returnvalue (Utilities|Array|Length _usable_distinct_item))
  (bind _returnvalue_2 (Transformation|GetWorldTransform _box))
  (bind _returnvalue_3 (Math|Random|RandomInteger _returnvalue))
  (bind _returnvalue_4 (Math|Transform|MakeTransform (.location _returnvalue_2) (.rotation _returnvalue_2)))
  (bind _returnvalue_5 (Game|SpawnActorfromClass "/Game/Blueprints/AI/BP_Customer.BP_Customer_C" _returnvalue_4 "AlwaysSpawn" "MultiplyWithRoot" 0 0))
  (bind _returnvalue_6 (Game|SpawnActorfromClass "/Game/Blueprints/AI/BP_CustomerController.BP_CustomerController_C" _returnvalue_4 "Undefined" "MultiplyWithRoot" 0 0))
  (Pawn|Possess _returnvalue_6 _returnvalue_5)
  (Variables|/Game/Blueprints/AI/BP_Customer.BP_Customer_C|SetExitArea _returnvalue_5 (Transformation|GetActorLocation))
  (Utilities|Array|AppendArray (Variables|Default|GetCustomers) (Utilities|Array|MakeArray _returnvalue_6))
  (Variables|/Game/Blueprints/AI/BP_CustomerController.BP_CustomerController_C|SetSpawner _returnvalue_6 self)
  (if (> _returnvalue 0)
    (Variables|/Game/Blueprints/AI/BP_CustomerController.BP_CustomerController_C|SetDistinct%20Item _returnvalue_6 (Utilities|Array|Get(acopy) _usable_distinct_item _returnvalue_3))
    (Utilities|Array|RemoveIndex _usable_distinct_item _returnvalue_3)
    (else
      (Development|PrintString "WARNING: Out of distinctive items"))))

(event Collision|EventActorBeginOverlap
  (params (OtherActor :type Actor%20Object%20Reference))
  (Variables|Default|SetOverlapping true))

(event EventTick
  (params (DeltaSeconds :type Float%20%28single-precision%29))
  (bind _usable_distinct_item (Variables|Default|GetUsable%20Distinct%20Item))
  (bind _box (Variables|Default|GetBox))
  (bind _returnvalue (Utilities|Array|Length _usable_distinct_item))
  (bind _returnvalue_2 (Transformation|GetWorldTransform _box))
  (bind _returnvalue_3 (Math|Random|RandomInteger _returnvalue))
  (bind _returnvalue_4 (Math|Transform|MakeTransform (.location _returnvalue_2) (.rotation _returnvalue_2)))
  (if (and (not (Variables|Default|GetOverlapping)) (< (Utilities|Array|Length (Variables|Default|GetCustomers)) (Variables|Default|GetMax%20Customers)))
    (Variables|Default|SetOverlapping true)
    (Utilities|FlowControl|Delay (Variables|Default|GetCustomer%20Spawn%20Time))
    (bind _returnvalue_5 (Game|SpawnActorfromClass "/Game/Blueprints/AI/BP_Customer.BP_Customer_C" _returnvalue_4 "AlwaysSpawn" "MultiplyWithRoot" 0 0))
    (bind _returnvalue_6 (Game|SpawnActorfromClass "/Game/Blueprints/AI/BP_CustomerController.BP_CustomerController_C" _returnvalue_4 "Undefined" "MultiplyWithRoot" 0 0))
    (Pawn|Possess _returnvalue_6 _returnvalue_5)
    (Variables|/Game/Blueprints/AI/BP_Customer.BP_Customer_C|SetExitArea _returnvalue_5 (Transformation|GetActorLocation))
    (Utilities|Array|AppendArray (Variables|Default|GetCustomers) (Utilities|Array|MakeArray _returnvalue_6))
    (Variables|/Game/Blueprints/AI/BP_CustomerController.BP_CustomerController_C|SetSpawner _returnvalue_6 self)
    (if (> _returnvalue 0)
      (Variables|/Game/Blueprints/AI/BP_CustomerController.BP_CustomerController_C|SetDistinct%20Item _returnvalue_6 (Utilities|Array|Get(acopy) _usable_distinct_item _returnvalue_3))
      (Utilities|Array|RemoveIndex _usable_distinct_item _returnvalue_3)
      (else
        (Development|PrintString "WARNING: Out of distinctive items")))))

(event Collision|EventActorEndOverlap
  (params (OtherActor :type Actor%20Object%20Reference))
  (Variables|Default|SetOverlapping false))

(fn ConstructionScript)

(fn FreeUsedItem
  (params (Distinct%20Item :type Actor%20Class%20Reference))
  (Utilities|Array|AddUnique (Variables|Default|GetUsable%20Distinct%20Item) Distinct%20Item))