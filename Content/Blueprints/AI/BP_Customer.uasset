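; BP_Customer is an AI customer that can detect and grab items, with its decisions left to an AI controller.
; An overlap on ItemGrabRange reports any BP_ItemBase to the controller stored through SetController.
; GrabItem passes the item, the customer's mesh and a physics constraint to a shared Grab call.
; SetSocketContent swaps the static mesh shown on the DistinctItem component.
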(event OnComponentBeginOverlap(ItemGrabRange)
  (params (OverlappedComponent :type Primitive%20Component%20Object%20Reference) (OtherActor :type Actor%20Object%20Reference) (OtherComp :type Primitive%20Component%20Object%20Reference) (OtherBodyIndex :type Integer) (bFromSweep :type Boolean) (SweepResult :type Hit%20Result%20Structure%20%28by%20ref%29))
  (bind _aicontroller (Variables|Default|GetAIController))
  (bind _asbp_item_base (Utilities|Casting|CastToBP_ItemBase OtherActor))
  (Utilities|IsValid _aicontroller
    (:Is%20Valid
      (Default|OnIteminRange _aicontroller _asbp_item_base))))

(event EventBeginPlay
  (|CallParentFunction) ; This node is disabled and will not be called.\nDrag off pins to build functionality.
)

(event Collision|EventActorBeginOverlap
  (params (OtherActor :type Actor%20Object%20Reference)))

(event EventTick
  (params (DeltaSeconds :type Float%20%28single-precision%29)))

(fn ConstructionScript
  (|CallParentFunction))

(fn SetController
  (params (Controller :type BP%20Customer%20Controller%20Object%20Reference))
  (Variables|Default|SetAIController Controller))

(fn GrabItem
  (params (Item :type BP%20Item%20Base%20Object%20Reference))
  (CallFunction|Grab Item (Variables|Character|GetMesh) (Variables|Default|GetPhysicsConstraint)))

(fn SetSocketContent
  (params (StaticMesh :type Static%20Mesh%20Object%20Reference))
  (Components|StaticMesh|SetStaticMesh (Variables|Default|GetDistinctItem) StaticMesh))